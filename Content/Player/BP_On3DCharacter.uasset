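; Player character Blueprint that tracks Health and handles death.
; CalculateDamage subtracts incoming damage from Health and has the controller unpossess the character once Health reaches zero or below.
; IsDead reports whether Health is at or below zero.
; The event graph holds only disabled placeholder events, and the construction script is empty.
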(event EventBeginPlay)

(event Collision|EventActorBeginOverlap
  (params (OtherActor :type Actor%20Object%20Reference)))

(event EventTick
  (params (DeltaSeconds :type Float%20%28single-precision%29)))

(event Input|ActionEvents|InputActionKnock
  (params (Key :type Key%20Structure :default "None")))

(fn ConstructionScript)

(fn IsDead
  (return (<= (Variables|Default|GetHealth) 0)))

(fn CalculateDamage
  (params (Damage :type Integer))
  (bind _output_get (Variables|Default|SetHealth (- (Variables|Default|GetHealth) Damage)))
  (if (<= _output_get 0)
    (Pawn|UnPossess (Pawn|GetController))))