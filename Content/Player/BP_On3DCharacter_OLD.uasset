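; Legacy 3D player character Blueprint that handles melee attacks and health-based death.
; The MeleeAttack event casts the mesh's anim instance to ABP_On3DCharacter and calls its Attack function.
; CalculateDamage subtracts damage from the health variable, then uses IsDead to check for zero or less and unpossesses the controller on death.
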(event EventMeleeAttack
  (bind _asabp_on_3dcharacter (Utilities|Casting|CastToABP_On3DCharacter (Components|SkeletalMesh|GetAnimInstance (Variables|Character|GetMesh))))
  (Utilities|IsValid _asabp_on_3dcharacter
    (:Is%20Valid
      (Default|Attack _asabp_on_3dcharacter))))

(event Input|ActionEvents|InputActionKnock
  (params (Key :type Key%20Structure :default "None")))

(fn ConstructionScript)

(fn IsDead
  (return (<= (Variables|Default|GetHealth_0) 0)))

(fn CalculateDamage
  (params (Damage :type Integer))
  (Variables|Default|SetHealth_0 (- (Variables|Default|GetHealth_0) Damage))
  (bind _dead (CallFunction|IsDead))
  (if _dead
    (Pawn|UnPossess (Pawn|GetController))))